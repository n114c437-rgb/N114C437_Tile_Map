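; BP_ParallaxBG is a side-scrolling background actor that creates a parallax effect as the player moves along X.
; On BeginPlay it caches player 0's character and starting X, plus the relative X of the far, mid and near background components.
; Each Tick it offsets every layer opposite the player's travel by a depth-scaled factor, moving nearer layers faster and pinning each to its own fixed Y depth.
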(event EventBeginPlay
  (bind _output_get (Variables|Default|SetPlayerRef (Game|GetPlayerCharacter 0)))
  (Variables|Default|SetPlayerStartX (.x (Transformation|GetActorLocation _output_get)))
  (Variables|Default|SetMidStartX (.x (Variables|/Script/Engine.SceneComponent|GetRelativeLocation (Variables|Default|GetBG_Mid))))
  (Variables|Default|SetFarStartX (.x (Variables|/Script/Engine.SceneComponent|GetRelativeLocation (Variables|Default|GetBG_Far))))
  (Variables|Default|SetNearStartX (.x (Variables|/Script/Engine.SceneComponent|GetRelativeLocation (Variables|Default|GetBG_Near)))))

(event Collision|EventActorBeginOverlap
  (params (OtherActor :type Actor%20Object%20Reference)))

(event EventTick
  (params (DeltaSeconds :type Float%20%28single-precision%29))
  (bind _playerref (Variables|Default|GetPlayerRef)
    (:then
      (Transformation|SetRelativeLocation (Variables|Default|GetBG_Far) (Math|Vector|MakeVector (+ (* (- (.x (Transformation|GetActorLocation _playerref)) (Variables|Default|GetPlayerStartX)) -0.09) (Variables|Default|GetFarStartX)) -3e+01 0.0) false false)
      (Transformation|SetRelativeLocation (Variables|Default|GetBG_Mid) (Math|Vector|MakeVector (+ (* (- (.x (Transformation|GetActorLocation _playerref)) (Variables|Default|GetPlayerStartX)) -0.3) (Variables|Default|GetMidStartX)) -2e+01 0.0) false false)
      (Transformation|SetRelativeLocation (Variables|Default|GetBG_Near) (Math|Vector|MakeVector (+ (* (- (.x (Transformation|GetActorLocation _playerref)) (Variables|Default|GetPlayerStartX)) -0.8) (Variables|Default|GetNearStartX)) -1e+01 0.0) false false))
    (:else)))

(fn ConstructionScript)